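; GameControllerBP is a game controller Blueprint that sets up the HUD and applies the effects of pickups.
; On BeginPlay it creates the HUD widget, adds it to the viewport, and caches the player pawn as PlayerBp.
; OnPickup branches on the pickup's class by chained casts: gems call ScaleControl on the player, rings increment RingsCollected, and healthmeme pickups call their own GainHP.
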(event EventBeginPlay
  (bind _returnvalue (UserInterface|CreateWidget "/Game/Blueprint/HUD/HUD.HUD_C"))
  (bind _output_get (Variables|Default|SetHUDReference _returnvalue))
  (UserInterface|Viewport|AddtoViewport _output_get 0)
  (bind _asplayer_bp (Utilities|Casting|CastToPlayerBp (Game|Player|GetPlayerPawn 0)))
  (Variables|Default|SetPlayerBP _asplayer_bp))

(fn ConstructionScript)

(fn OnPickup
  (params (PickUpType :type Actor%20Object%20Reference))
  (Utilities|Casting|CastTobpPickUpGem PickUpType
    (:then
      (Default|ScaleControl (Variables|Default|GetPlayerBP) true))
    (:CastFailed
      (Utilities|Casting|CastTobpPickUpRing PickUpType
        (:then
          (Variables|Default|SetRingsCollected (+ (Variables|Default|GetRingsCollected) 1)))
        (:CastFailed
          (bind _ashealthmeme (Utilities|Casting|CastTohealthmeme PickUpType))
          (Default|GainHP _ashealthmeme))))))