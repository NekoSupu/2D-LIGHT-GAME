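; Follow camera actor that tracks the first player's pawn at a world offset with a fixed rotation.
; Each Tick it sets its transform with TInterpTo toward the pawn location plus WorldOffest.
; The interpolation start takes X from the pawn, so X locks instantly while Y and Z ease.
; WorldOffest is also added to that start point every frame, shifting where Y and Z settle.
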(event EventTick
  (params (DeltaSeconds :type Float%20%28single-precision%29))
  (bind _returnvalue (Game|Player|GetPlayerPawn 0))
  (bind _returnvalue_2 (Transformation|GetActorTransform))
  (bind _location (Math|Transform|BreakTransform _returnvalue_2))
  (bind _returnvalue_3 (Transformation|GetActorTransform _returnvalue))
  (Utilities|IsValid _returnvalue
    (:Is%20Valid
      (Transformation|SetActorTransform (Class|KismetMathLibrary|TInterpto (Math|Transform|MakeTransform (+ (Math|Vector|MakeVector (.x (.Location (Math|Transform|BreakTransform _returnvalue_3))) (.y _location) (.z _location)) (Variables|Default|GetWorldOffest)) "0,-90.000000, 0" "1,1,1.000000") (Math|Transform|MakeTransform (+ (.Location (Math|Transform|BreakTransform _returnvalue_3)) (Variables|Default|GetWorldOffest)) "0,-90.000000, 0") DeltaSeconds 3.0)))))

(fn ConstructionScript)