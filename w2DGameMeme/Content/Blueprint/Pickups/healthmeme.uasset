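; Health pickup Blueprint that a player consumes by walking into it while below full health.
; An InnerCollision overlap with PlayerBp checks health, reports the pickup to that player's GameController, then destroys the actor.
; A separate GainHP event, not called within this graph, adds a fixed, unclamped heal to player 0.
; BeginPlay caches the GameControllerBP game mode, though the overlap uses the player's own reference.
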(event OnComponentBeginOverlap(InnerCollision)
  (params (OverlappedComponent :type Primitive%20Component%20Object%20Reference) (OtherActor :type Actor%20Object%20Reference) (OtherComp :type Primitive%20Component%20Object%20Reference) (OtherBodyIndex :type Integer) (bFromSweep :type Boolean) (SweepResult :type Hit%20Result%20Structure%20%28by%20ref%29))
  (bind _asplayer_bp (Utilities|Casting|CastToPlayerBp OtherActor))
  (if (> 1e+02 (Variables|/Game/Blueprint/Player/PlayerBp.PlayerBp_C|GetHealth _asplayer_bp))
    (Default|OnPickup (Variables|/Game/Blueprint/Player/PlayerBp.PlayerBp_C|GetGameController _asplayer_bp) self)
    (Actor|DestroyActor)))

(event Custom|GainHP
  (bind _asplayer_bp (Utilities|Casting|CastToPlayerBp (Game|GetPlayerCharacter 0)))
  (Variables|/Game/Blueprint/Player/PlayerBp.PlayerBp_C|SetHealth _asplayer_bp (+ (Variables|/Game/Blueprint/Player/PlayerBp.PlayerBp_C|GetHealth _asplayer_bp) 25.0)))

(event EventBeginPlay
  (bind _asgame_controller_bp (Utilities|Casting|CastToGameControllerBP (Game|GetGameMode)))
  (Variables|Default|SetGamerControllerBP _asgame_controller_bp))

(fn ConstructionScript)