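; Arrow trap actor that spawns a BpArrow every second while moving vertically.
; On BeginPlay it stores its start location and starts both a looping Fire timer and the Movement timeline.
; The timeline lerps the actor along Z from that start, with the Speed variable acting as the travel offset rather than a rate.
; Each Fire spawns the arrow at the SpawnPoint component's world transform.
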(event Custom|Fire
  (Game|SpawnActorfromClass "/Game/Blueprint/Misc/bpArrow.bpArrow_C" (Transformation|GetWorldTransform (Variables|Default|GetSpawn%20Point)) "Undefined" 0 0))

(event EventBeginPlay
  (Variables|Default|SetStartpos (Transformation|GetActorLocation))
  (Utilities|Time|SetTimerbyFunctionName 0 "Fire" 1.0 true)
  (bind _move (Timeline|Movement PlayFromStart)
    (:Update
      (Transformation|SetActorLocation (Math|Vector|Lerp(Vector) (Variables|Default|GetStartpos) (Math|Vector|MakeVector (.x (Variables|Default|GetStartpos)) (.y (Variables|Default|GetStartpos)) (+ (.z (Variables|Default|GetStartpos)) (Variables|Default|GetSpeed))) _move) false false))))

(fn ConstructionScript)