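; A moving platform Blueprint that shifts itself between its starting location and an offset point.
; On BeginPlay it stores its location and plays the Movement timeline, whose Move track drives a lerp to the start plus the Speed vector.
; Despite its name, Speed acts as a travel offset, and the location is set without sweep.
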(event EventBeginPlay
  (bind _speed (Variables|Default|GetSpeed))
  (Variables|Default|SetStartpos (Transformation|GetActorLocation))
  (bind _move (Timeline|Movement PlayFromStart)
    (:Update
      (Transformation|SetActorLocation (Math|Vector|Lerp(Vector) (Variables|Default|GetStartpos) (Math|Vector|MakeVector (+ (.x (Variables|Default|GetStartpos)) (.x _speed)) (+ (.y (Variables|Default|GetStartpos)) (.y _speed)) (+ (.z (Variables|Default|GetStartpos)) (.z _speed))) _move) false false))))

(fn ConstructionScript)